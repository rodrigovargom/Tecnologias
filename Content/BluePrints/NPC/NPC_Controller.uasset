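; AI controller for an NPC that fills its blackboard on BeginPlay, then runs its behavior tree.
; It scans every PathPoint_Blueprint and stores the locations of those whose Mensaje matches Cerca (near) or Lejos (far) as CercaLocation and LejosLocation.
; The first ControlledObject found in the level becomes the Enemy key, and NPC_BehaviorTree starts after a short delay.
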(event EventBeginPlay
  (bind _self self)
  (bind _returnvalue (AI|GetBlackboard _self))
  (Class|AIController|UseBlackboard "/Game/BluePrints/NPC/NPC_Blackboard.NPC_Blackboard")
  (Utilities|FlowControl|Sequence
    (:then_0
      (bind _outactors (Actor|GetAllActorsOfClass "/Game/BluePrints/PathPoint_Blueprint.PathPoint_Blueprint_C"))
      (for _array_element _outactors
        (bind _aspath_point_blueprint (Utilities|Casting|CastToPathPoint_Blueprint _array_element))
        (bind _output_get (Variables|Default|SetcurrentPoint%20 _aspath_point_blueprint))
        (if (Utilities|Enum|Equal(Enum) (Variables|Default|GetCerca) (Variables|/Game/BluePrints/PathPoint_Blueprint.PathPoint_Blueprint_C|GetMensaje _output_get))
          (AI|Components|Blackboard|SetValueasVector _returnvalue (Utilities|Name|MakeLiteralName "CercaLocation") (Transformation|GetActorLocation (Variables|Default|GetcurrentPoint%20)))
          (elif (Utilities|Enum|Equal(Enum) (Variables|/Game/BluePrints/PathPoint_Blueprint.PathPoint_Blueprint_C|GetMensaje _output_get) (Variables|Default|GetLejos))
            (AI|Components|Blackboard|SetValueasVector _returnvalue (Utilities|Name|MakeLiteralName "LejosLocation") (Transformation|GetActorLocation (Variables|Default|GetcurrentPoint%20)))))))
    (:then_1
      (bind _outactors_2 (Actor|GetAllActorsOfClass "/Game/Ejercicio/ControlledObject.ControlledObject_C"))
      (AI|Components|Blackboard|SetValueasObject (AI|GetBlackboard self) (Variables|Default|GetEnemy) (Utilities|Array|Get(acopy) _outactors_2))
      (Utilities|FlowControl|Delay 1.0)
      (AI|RunBehaviorTree "/Game/BluePrints/NPC/NPC_BehaviorTree.NPC_BehaviorTree"))))

(fn ConstructionScript)